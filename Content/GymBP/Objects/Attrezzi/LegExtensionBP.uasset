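; Leg extension gym machine that NPCs use through the parent class's StartInteraction and EndInteraction events.
; On start it disables machine collision and eases the NPC onto a seat marker while the looping machine animation and character montage begin in parallel.
; When the montage completes, it stops the machine, moves the NPC to an exit marker raised by capsule half-height, and restores collision.
; A completion flag gates the parent's EndInteraction.
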(event `/Game/Interfaces/InteractGym.StartInteraction`
  (params (InteractingActor :type "Actor Object Reference"))
  (bind _character (`self.Character`))
  (bind _characterlocation (`self.CharacterLocation`))
  (bind (_returnvalue_x _returnvalue_y _returnvalue_z) (`KismetMathLibrary.BreakVector` (`SceneComponent.K2_GetComponentLocation` _characterlocation)))
  (bind _rootcomponent (`Actor.RootComponent` (`self.InteractingActor`)))
  (`parent.StartInteraction` InteractingActor)
  (bind _asnpc_bp (cast `/Game/GymBP/NPC/AI/NPC_BP` (`self.InteractingActor`)))
  (bind _output_get (set `self.Character` _asnpc_bp))
  (`|ExecutionSequence`
    (:`then_0`
      (`PrimitiveComponent.SetCollisionEnabled` (`self.StaticMesh`) "NoCollision")
      (`PrimitiveComponent.SetCollisionEnabled` (`self.SkeletalMeshMacchina`) "NoCollision")
      (`KismetSystemLibrary.MoveComponentTo` _rootcomponent (`KismetMathLibrary.MakeVector` _returnvalue_x _returnvalue_y _returnvalue_z) (`SceneComponent.K2_GetComponentRotation` _characterlocation) true true 0.5 true))
    (:`then_1`
      (`SkeletalMeshComponent.PlayAnimation` (`self.SkeletalMeshMacchina`) "/Game/Assetfore/OMINOEATTREZZO/LegExtension/LEG_EXTENSION_anim.LEG_EXTENSION_anim" true)
      (`|PlayMontage` (`Character.Mesh` _output_get) "/Game/Assetfore/OMINOEATTREZZO/LegExtension/LegExtensionANIMMONTAGE.LegExtensionANIMMONTAGE"
        (:`OnCompleted`
          (`SkeletalMeshComponent.Stop` (`self.SkeletalMeshMacchina`))
          (`KismetSystemLibrary.MoveComponentTo` _rootcomponent (+ (`SceneComponent.K2_GetComponentLocation` (`self.CharacterLocationFinale`)) (`KismetMathLibrary.MakeVector` 0.0 0.0 (`CapsuleComponent.CapsuleHalfHeight` (`Character.CapsuleComponent` _character)))) (`self.K2_GetActorRotation` _character) true true 0.2 true)
          (`PrimitiveComponent.SetCollisionEnabled` (`self.StaticMesh`) "QueryAndPhysics")
          (`PrimitiveComponent.SetCollisionEnabled` (`self.SkeletalMeshMacchina`) "QueryAndPhysics")
          (set `self.AzioneCompletata` true)
          (`/Game/Interfaces/InteractGym.EndInteraction`))))))

(event `/Game/Interfaces/InteractGym.EndInteraction`
  (if (`self.AzioneCompletata`)
    (`parent.EndInteraction`)))

(fn `UserConstructionScript`
  (`parent.UserConstructionScript`))