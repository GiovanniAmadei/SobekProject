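; Interactable gym treadmill Blueprint that has the interacting character play a running animation.
; On interaction start, it eases the character's root onto the treadmill's location marker, offset by capsule half-height, while the montage starts alongside.
; When the montage completes, it begins moving the character to the end marker, flags the action complete and immediately ends the interaction.
; EndInteraction reaches the parent only once that flag is set, which is never reset here.
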(event `/Game/Interfaces/InteractGym.StartInteraction`
  (params (InteractingActor :type "Character Object Reference"))
  (bind _characterendlocation (`self.CharacterEndLocation`))
  (bind _characterlocation (`self.CharacterLocation`))
  (bind (_returnvalue_x _returnvalue_y _returnvalue_z) (`KismetMathLibrary.BreakVector` (`SceneComponent.K2_GetComponentLocation` _characterlocation)))
  (bind (_returnvalue_x_2 _returnvalue_y_2 _returnvalue_z_2) (`KismetMathLibrary.BreakVector` (`SceneComponent.K2_GetComponentLocation` _characterendlocation)))
  (`parent.StartInteraction` InteractingActor)
  (bind _output_get (set `self.Character_0` (`self.InteractingActor`)))
  (`|ExecutionSequence`
    (:`then_0`
      (`KismetSystemLibrary.MoveComponentTo` (`Actor.RootComponent` (`self.InteractingActor`)) (`KismetMathLibrary.MakeVector` _returnvalue_x _returnvalue_y (+ _returnvalue_z (`CapsuleComponent.CapsuleHalfHeight` (`Character.CapsuleComponent` (`self.Character_0`))))) (`SceneComponent.K2_GetComponentRotation` _characterlocation) true true 0.5))
    (:`then_1`
      (`|PlayMontage` (`Character.Mesh` _output_get) "/Game/Assetfore/animazioni/AnimMontages/CORSAMONTAGE.CORSAMONTAGE"
        (:`OnCompleted`
          (`KismetSystemLibrary.MoveComponentTo` (`Actor.RootComponent` (`self.Character_0`)) (`KismetMathLibrary.MakeVector` _returnvalue_x_2 _returnvalue_y_2 _returnvalue_z_2) (`SceneComponent.K2_GetComponentRotation` _characterendlocation) true true 0.5)
          (set `self.AzioneCompletata` true)
          (`/Game/Interfaces/InteractGym.EndInteraction`))))))

(event `/Game/Interfaces/InteractGym.EndInteraction`
  (if (`self.AzioneCompletata`)
    (`parent.EndInteraction`)))

(fn `UserConstructionScript`
  (`parent.UserConstructionScript`))