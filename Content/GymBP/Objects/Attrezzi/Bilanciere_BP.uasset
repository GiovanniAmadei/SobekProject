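; Barbell gym equipment that an NPC_BP character uses to perform a squat animation.
; On interaction start it disables the bar's collision, eases the NPC to the CharacterLocation marker and plays the Squat montage.
; Montage notifies drive the bar: "Prendi" attaches it to the left hand socket and eases it in, while any other notify reattaches it to the Scene component.
; Ending the interaction only runs the parent logic.
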(event `self.IniziaInterazione`
  (bind _characterlocation (`self.CharacterLocation`))
  (bind _staticmesh (`self.StaticMesh`))
  (bind (_returnvalue_x _returnvalue_y _returnvalue_z) (`KismetMathLibrary.BreakVector` (`SceneComponent.K2_GetComponentLocation` _characterlocation)))
  (`parent.IniziaInterazione`)
  (bind _asnpc_bp (cast `/Game/GymBP/NPC/AI/NPC_BP` (`self.InteractingActor`)))
  (bind _output_get (set `self.Character` _asnpc_bp))
  (`PrimitiveComponent.SetCollisionEnabled` (`self.StaticMesh`) "NoCollision")
  (`|ExecutionSequence`
    (:`then_0`
      (`KismetSystemLibrary.MoveComponentTo` (`Actor.RootComponent` (`self.InteractingActor`)) (`KismetMathLibrary.MakeVector` _returnvalue_x _returnvalue_y (+ _returnvalue_z (`CapsuleComponent.CapsuleHalfHeight` (`Character.CapsuleComponent` (`self.Character`))))) (`SceneComponent.K2_GetComponentRotation` _characterlocation) true true 0.5))
    (:`then_1`
      (bind _notifyname (`|PlayMontage` (`Character.Mesh` _output_get) "/Game/Assetfore/animazioni/AnimMontages/Squat.Squat")
        (:`OnNotifyBegin`
          (if (== _notifyname "Prendi")
            (`SceneComponent.K2_AttachToComponent` _staticmesh (`Character.Mesh` (`self.Character`)) "LeftHandSocket" "KeepWorld" "KeepWorld" "KeepWorld" true)
            (`KismetSystemLibrary.MoveComponentTo` _staticmesh (0.0 0.0 0.0) (struct) true true)
            (else
              (`SceneComponent.K2_AttachToComponent` _staticmesh (`self.Scene`) "None" "KeepWorld" "KeepWorld" "KeepWorld" true))))))))

(event `self.FinisciInterazione`
  (`parent.FinisciInterazione`))

(fn `UserConstructionScript`
  (`parent.UserConstructionScript`))