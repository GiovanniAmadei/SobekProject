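; Interactable gym dumbbell prop that an NPC uses to perform a curl exercise.
; On interaction it disables mesh collision, eases the NPC to a marker and plays the curl montage.
; Montage notifies drive the handoff: "Inizio" attaches both meshes to hand sockets, others reattach them to Scene and move Scene using transforms saved at BeginPlay.
; Montage completion sets a flag that lets EndInteraction reach the parent logic.
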(event `self.ReceiveBeginPlay`
  (`parent.ReceiveBeginPlay`)
  (set `self.OriginalTransform` (`SceneComponent.K2_GetComponentToWorld` (`self.StaticMesh`)))
  (set `self.OriginalTransform1` (`SceneComponent.K2_GetComponentToWorld` (`self.StaticMesh1`))))

(event `/Game/Interfaces/InteractGym.StartInteraction`
  (params (InteractingActor :type "Actor Object Reference"))
  (bind _staticmesh (`self.StaticMesh`))
  (bind (_originaltransform_location _originaltransform_rotation) (`KismetMathLibrary.BreakTransform` (`self.OriginalTransform`)))
  (bind _characterlocation (`self.CharacterLocation`))
  (bind _staticmesh1 (`self.StaticMesh1`))
  (bind _scene (`self.Scene`))
  (bind (_originaltransform1_location _originaltransform1_rotation) (`KismetMathLibrary.BreakTransform` (`self.OriginalTransform1`)))
  (bind (_returnvalue_x _returnvalue_y _returnvalue_z) (`KismetMathLibrary.BreakVector` (`SceneComponent.K2_GetComponentLocation` _characterlocation)))
  (bind _mesh (`Character.Mesh` (`self.Character`)))
  (`parent.StartInteraction` InteractingActor)
  (bind _asnpc_bp (cast `/Game/GymBP/NPC/AI/NPC_BP` (`self.InteractingActor`)))
  (bind _output_get (set `self.Character` _asnpc_bp))
  (`PrimitiveComponent.SetCollisionEnabled` (`self.StaticMesh`) "NoCollision")
  (`PrimitiveComponent.SetCollisionEnabled` (`self.StaticMesh1`) "NoCollision")
  (`|ExecutionSequence`
    (:`then_0`
      (`KismetSystemLibrary.MoveComponentTo` (`Actor.RootComponent` (`self.InteractingActor`)) (`KismetMathLibrary.MakeVector` _returnvalue_x _returnvalue_y (+ _returnvalue_z (`CapsuleComponent.CapsuleHalfHeight` (`Character.CapsuleComponent` (`self.Character`))))) (`SceneComponent.K2_GetComponentRotation` _characterlocation) true true 0.5))
    (:`then_1`
      (bind _notifyname (`|PlayMontage` (`Character.Mesh` _output_get) "/Game/Assetfore/animazioni/AnimMontages/CURLMontage.CURLMontage")
        (:`OnCompleted`
          (set `self.AzioneCompletata` true)
          (`/Game/Interfaces/InteractGym.EndInteraction`))
        (:`OnNotifyBegin`
          (if (== _notifyname "Inizio")
            (`StaticMeshComponent.SetStaticMesh` (`self.StaticMesh`) (`StaticMeshComponent.StaticMesh` (`self.StaticMesh1`)))
            (`SceneComponent.K2_AttachToComponent` _staticmesh1 _mesh "LeftHandSocket" "KeepWorld" "KeepWorld" "KeepWorld" true)
            (`KismetSystemLibrary.MoveComponentTo` _staticmesh1 (0.0 0.0 0.0) (struct) true true)
            (`SceneComponent.K2_AttachToComponent` _staticmesh _mesh "RightHandSocket" "KeepWorld" "KeepWorld" "KeepWorld" true)
            (`KismetSystemLibrary.MoveComponentTo` _staticmesh (0.0 0.0 0.0) (struct) true true)
            (else
              (`StaticMeshComponent.SetStaticMesh` (`self.StaticMesh`) (`StaticMeshComponent.StaticMesh` (`self.StaticMesh1`)))
              (`SceneComponent.K2_AttachToComponent` _staticmesh1 _scene "LeftHandSocket" "KeepWorld" "KeepWorld" "KeepWorld" true)
              (`KismetSystemLibrary.MoveComponentTo` _scene _originaltransform1_location _originaltransform1_rotation true true)
              (`SceneComponent.K2_AttachToComponent` _staticmesh _scene "RightHandSocket" "KeepWorld" "KeepWorld" "KeepWorld" true)
              (`KismetSystemLibrary.MoveComponentTo` _scene _originaltransform_location _originaltransform_rotation true true))))))))

(event `/Game/Interfaces/InteractGym.EndInteraction`
  (if (`self.AzioneCompletata`)
    (`parent.EndInteraction`)))

(fn `UserConstructionScript`
  (`parent.UserConstructionScript`))