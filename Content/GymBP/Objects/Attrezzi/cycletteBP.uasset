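; Gym exercise bike (cyclette) object that NPCs use through an inherited interaction event (IniziaInterazione).
; After the parent logic, it proceeds only for an NPC_BP actor and sets its static mesh collision to query and physics.
; It eases the NPC onto the CharacterPosition transform, raised by the capsule half height, while a Sequence starts the cycling montage without waiting for the move to finish.
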(event `self.IniziaInterazione`
  (bind _character_position (`self.character position`))
  (bind (_returnvalue_x _returnvalue_y _returnvalue_z) (`KismetMathLibrary.BreakVector` (`SceneComponent.K2_GetComponentLocation` _character_position)))
  (`parent.IniziaInterazione`)
  (bind _asnpc_bp (cast `/Game/GymBP/NPC/AI/NPC_BP` (`self.InteractingActor`)))
  (bind _output_get (set `self.Character_0` _asnpc_bp))
  (`PrimitiveComponent.SetCollisionEnabled` (`self.StaticMesh`) "QueryAndPhysics")
  (`|ExecutionSequence`
    (:`then_0`
      (`KismetSystemLibrary.MoveComponentTo` (`Actor.RootComponent` (`self.InteractingActor`)) (`KismetMathLibrary.MakeVector` _returnvalue_x _returnvalue_y (+ _returnvalue_z (`CapsuleComponent.CapsuleHalfHeight` (`Character.CapsuleComponent` (`self.Character_0`))))) (`SceneComponent.K2_GetComponentRotation` _character_position) true true 0.5))
    (:`then_1`
      (`|PlayMontage` (`Character.Mesh` _output_get) "/Game/Assetfore/animazioni/AnimMontages/CycletteMONTAGE.CycletteMONTAGE"))))

(fn `UserConstructionScript`
  (`parent.UserConstructionScript`))