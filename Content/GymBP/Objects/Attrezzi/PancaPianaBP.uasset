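; Flat bench press gym equipment that an NPC uses through the inherited interaction events.
; On interaction it disables mesh collision, eases the NPC onto the bench and plays the bench press montage.
; Montage notifies drive the barbell: "Inizio" attaches it to the character's socket, any other returns it to its BeginPlay transform and moves the NPC to the exit point.
; The parent's end-interaction logic runs only once the montage completes.
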(event `self.ReceiveBeginPlay`
  (`parent.ReceiveBeginPlay`)
  (set `self.TransformLocation` (`SceneComponent.K2_GetComponentToWorld` (`self.Bilanciere`))))

(event `/Game/Interfaces/InteractGym.StartInteraction`
  (params (InteractingActor :type "Actor Object Reference"))
  (bind (_transformlocation_location _transformlocation_rotation) (`KismetMathLibrary.BreakTransform` (`self.TransformLocation`)))
  (bind _characterlocation (`self.CharacterLocation`))
  (bind _bilanciere (`self.Bilanciere`))
  (bind _character (`self.Character`))
  (bind (_returnvalue_x _returnvalue_y _returnvalue_z) (`KismetMathLibrary.BreakVector` (`SceneComponent.K2_GetComponentLocation` _characterlocation)))
  (`parent.StartInteraction` InteractingActor)
  (bind _asnpc_bp (cast `/Game/GymBP/NPC/AI/NPC_BP` (`self.InteractingActor`)))
  (bind _output_get (set `self.Character` _asnpc_bp))
  (`PrimitiveComponent.SetCollisionEnabled` (`self.StaticMesh`) "NoCollision")
  (`|ExecutionSequence`
    (:`then_0`
      (`KismetSystemLibrary.MoveComponentTo` (`Actor.RootComponent` (`self.InteractingActor`)) (`KismetMathLibrary.MakeVector` _returnvalue_x _returnvalue_y (+ _returnvalue_z (`CapsuleComponent.CapsuleHalfHeight` (`Character.CapsuleComponent` (`self.Character`))))) (`SceneComponent.K2_GetComponentRotation` _characterlocation) true true 0.5))
    (:`then_1`
      (bind _notifyname (`|PlayMontage` (`Character.Mesh` _output_get) "/Game/Assetfore/animazioni/AnimMontages/PANCAPIANAMONTAGE.PANCAPIANAMONTAGE")
        (:`OnCompleted`
          (set `self.AzioneCompletata` true)
          (`/Game/Interfaces/InteractGym.EndInteraction`))
        (:`OnNotifyBegin`
          (if (== _notifyname "Inizio")
            (`SceneComponent.K2_AttachToComponent` _bilanciere (`Character.Mesh` (`self.Character`)) "SocketBilancierePancaPiana" "KeepWorld" "KeepWorld" "KeepWorld" true)
            (`KismetSystemLibrary.MoveComponentTo` _bilanciere (0.0 0.0 0.0) (struct) true true)
            (else
              (`SceneComponent.K2_DetachFromComponent` _bilanciere "KeepWorld" "KeepWorld" "KeepWorld" true)
              (`KismetSystemLibrary.MoveComponentTo` _bilanciere _transformlocation_location _transformlocation_rotation true true)
              (`KismetSystemLibrary.MoveComponentTo` (`Actor.RootComponent` _character) (+ (`SceneComponent.K2_GetComponentLocation` (`self.CharacterEndLocation`)) (`KismetMathLibrary.MakeVector` 0.0 0.0 (`CapsuleComponent.CapsuleHalfHeight` (`Character.CapsuleComponent` _character)))) (`self.K2_GetActorRotation` _character) true true))))))))

(event `/Game/Interfaces/InteractGym.EndInteraction`
  (if (`self.AzioneCompletata`)
    (`parent.EndInteraction`)))

(fn `UserConstructionScript`
  (`parent.UserConstructionScript`))