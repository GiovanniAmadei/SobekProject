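; LatLiberaBP is an interactable gym machine that an NPC_BP character uses through the inherited StartInteraction and EndInteraction events.
; On start it disables collision on its meshes and eases the NPC onto the machine, offset by capsule half-height, while a looping machine animation plays alongside the NPC's montage.
; When the montage completes, it stops the machine, moves the NPC to CharacterLocationFinale and sets AzioneCompletata, which gates the parent's EndInteraction.
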(event `/Game/Interfaces/InteractGym.StartInteraction`
  (params (InteractingActor :type "Actor Object Reference"))
  (bind _character (`self.Character`))
  (bind _skeletalmesh (`self.SkeletalMesh`))
  (bind (_returnvalue_x _returnvalue_y _returnvalue_z) (`KismetMathLibrary.BreakVector` (`SceneComponent.K2_GetComponentLocation` _skeletalmesh)))
  (bind _rootcomponent (`Actor.RootComponent` (`self.InteractingActor`)))
  (`parent.StartInteraction` InteractingActor)
  (bind _asnpc_bp (cast `/Game/GymBP/NPC/AI/NPC_BP` (`self.InteractingActor`)))
  (bind _output_get (set `self.Character` _asnpc_bp))
  (`|ExecutionSequence`
    (:`then_0`
      (`PrimitiveComponent.SetCollisionEnabled` (`self.StaticMesh`) "NoCollision")
      (`PrimitiveComponent.SetCollisionEnabled` (`self.SkeletalMesh1`) "NoCollision")
      (`KismetSystemLibrary.MoveComponentTo` _rootcomponent (`KismetMathLibrary.MakeVector` _returnvalue_x _returnvalue_y (+ _returnvalue_z (`CapsuleComponent.CapsuleHalfHeight` (`Character.CapsuleComponent` (`self.Character`))))) (`SceneComponent.K2_GetComponentRotation` _skeletalmesh) true true 0.5 true))
    (:`then_1`
      (`SkeletalMeshComponent.PlayAnimation` (`self.SkeletalMesh1`) "/Game/Assetfore/OMINOEATTREZZO/LATLIBERA/v2/LAT_LIBERA_2_anim.LAT_LIBERA_2_anim" true)
      (`|PlayMontage` (`Character.Mesh` _output_get) "/Game/Assetfore/OMINOEATTREZZO/LATLIBERA/v2/LatLiberaMontage.LatLiberaMontage"
        (:`OnCompleted`
          (`SkeletalMeshComponent.Stop` (`self.SkeletalMesh1`))
          (`KismetSystemLibrary.MoveComponentTo` _rootcomponent (+ (`SceneComponent.K2_GetComponentLocation` (`self.CharacterLocationFinale`)) (`KismetMathLibrary.MakeVector` 0.0 0.0 (`CapsuleComponent.CapsuleHalfHeight` (`Character.CapsuleComponent` _character)))) (`self.K2_GetActorRotation` _character) true true 0.2 true)
          (set `self.AzioneCompletata` true)
          (`/Game/Interfaces/InteractGym.EndInteraction`))))))

(event `/Game/Interfaces/InteractGym.EndInteraction`
  (if (`self.AzioneCompletata`)
    (`parent.EndInteraction`)))

(fn `UserConstructionScript`
  (`parent.UserConstructionScript`))