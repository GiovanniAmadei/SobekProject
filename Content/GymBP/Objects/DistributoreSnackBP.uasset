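; A gym snack vending machine Blueprint that a character can interact with, extending a parent interactable's start and end logic.
; On interaction it eases the character to the CharacterLocation point while playing the machine-use montage.
; When that montage completes it ends the interaction, gated by AzioneCompletata.
; If the user is an NPC_BP, it then plays a drinking montage with the bottle shown on a right-hand socket, hiding it afterwards.
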(event `/Game/Interfaces/InteractGym.StartInteraction`
  (params (InteractingActor :type "Character Object Reference"))
  (bind _characterlocation (`self.CharacterLocation`))
  (bind _interactingactor (`self.InteractingActor`))
  (bind (_returnvalue_x _returnvalue_y _returnvalue_z) (`KismetMathLibrary.BreakVector` (`SceneComponent.K2_GetComponentLocation` _characterlocation)))
  (`parent.StartInteraction` InteractingActor)
  (bind _output_get (set `self.Character` _interactingactor))
  (`|ExecutionSequence`
    (:`then_0`
      (`KismetSystemLibrary.MoveComponentTo` (`Actor.RootComponent` (`self.InteractingActor`)) (`KismetMathLibrary.MakeVector` _returnvalue_x _returnvalue_y (+ _returnvalue_z 10.0)) (`SceneComponent.K2_GetComponentRotation` _characterlocation) true true 0.5))
    (:`then_1`
      (`|PlayMontage` (`Character.Mesh` _output_get) "/Game/Assetfore/OmarinoSvilupparty/animazioni/MacchinetteAnimMontage.MacchinetteAnimMontage"
        (:`OnCompleted`
          (set `self.AzioneCompletata` true)
          (`/Game/Interfaces/InteractGym.EndInteraction`)
          (bind _asnpc_bp (cast `/Game/GymBP/NPC/AI/NPC_BP` _interactingactor))
          (bind _mesh (`Character.Mesh` _asnpc_bp))
          (`|PlayMontage` _mesh "/Game/Assetfore/OmarinoSvilupparty/animazioni/interazioni/bere/BereMontage.BereMontage"
            (:`then`
              (bind _bottiglia (`/Game/GymBP/NPC/AI/NPC_BP.Bottiglia` _asnpc_bp))
              (`SceneComponent.SetVisibility` _bottiglia true false)
              (`SceneComponent.K2_AttachToComponent` _bottiglia _mesh "RightHandSocketBorraccia" "KeepRelative" "KeepRelative" "KeepRelative" true))
            (:`OnCompleted`
              (`SceneComponent.SetVisibility` _bottiglia false false))))))))

(event `/Game/Interfaces/InteractGym.EndInteraction`
  (if (`self.AzioneCompletata`)
    (`parent.EndInteraction`)))

(fn `UserConstructionScript`
  (`parent.UserConstructionScript`))