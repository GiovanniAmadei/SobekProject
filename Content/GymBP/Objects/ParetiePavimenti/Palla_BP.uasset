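; Gym exercise ball interactable on which an NPC performs an abdominal workout.
; StartInteraction eases the NPC onto the equipment's character anchor, offset by capsule half-height, and starts the ball crunch montage.
; Montage completion sets a flag and calls EndInteraction, which passes to the parent only once that flag is set.
; SetCalendar and SetClock are stubs returning false.
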(event `/Game/Interfaces/InteractGym.StartInteraction`
  (params (InteractingActor :type "Actor Object Reference"))
  (bind _characterlocationattrezzo (`self.CharacterLocationAttrezzo`))
  (bind (_returnvalue_x _returnvalue_y _returnvalue_z) (`KismetMathLibrary.BreakVector` (`SceneComponent.K2_GetComponentLocation` _characterlocationattrezzo)))
  (`parent.StartInteraction` InteractingActor)
  (bind _asnpc_bp (cast `/Game/GymBP/NPC/AI/NPC_BP` (`self.InteractingActor`)))
  (bind _output_get (set `self.CharacterAzione` _asnpc_bp))
  (`|ExecutionSequence`
    (:`then_0`
      (`KismetSystemLibrary.MoveComponentTo` (`Actor.RootComponent` (`self.InteractingActor`)) (`KismetMathLibrary.MakeVector` _returnvalue_x _returnvalue_y (+ _returnvalue_z (`CapsuleComponent.CapsuleHalfHeight` (`Character.CapsuleComponent` (`self.CharacterAzione`))))) (`SceneComponent.K2_GetComponentRotation` _characterlocationattrezzo) true true 0.5))
    (:`then_1`
      (`|PlayMontage` (`Character.Mesh` _output_get) "/Game/Assetfore/OmarinoSvilupparty/animazioni/palla/AddominaliPallaANIMMONTAGE.AddominaliPallaANIMMONTAGE"
        (:`OnCompleted`
          (set `self.AzioneCompletata` true)
          (`/Game/Interfaces/InteractGym.EndInteraction`))))))

(event `/Game/Interfaces/InteractGym.EndInteraction`
  (if (`self.AzioneCompletata`)
    (`parent.EndInteraction`)))

(fn `SetCalendar`
  (params (Date :type "Array of Integer (by ref)"))
  (returns (Success :type Boolean))
  (return false))

(fn `SetClock`
  (params (Time :type "Array of Integer (by ref)"))
  (returns (Success :type Boolean))
  (return false))

(fn `UserConstructionScript`
  (`parent.UserConstructionScript`))