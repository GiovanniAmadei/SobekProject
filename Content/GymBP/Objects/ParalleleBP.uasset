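; Interactable parallel bars for the gym, which an NPC uses by playing an exercise montage.
; On interaction it disables mesh collision and eases the NPC to a start marker, offset by capsule half-height, while the montage plays.
; When the montage completes, it moves the NPC to a final marker, restores collision and ends the interaction.
; A completion flag blocks the parent's EndInteraction until the first montage has completed.
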(event `/Game/Interfaces/InteractGym.StartInteraction`
  (params (InteractingActor :type "Actor Object Reference"))
  (bind _characterlocation (`self.CharacterLocation`))
  (bind (_returnvalue_x _returnvalue_y _returnvalue_z) (`KismetMathLibrary.BreakVector` (`SceneComponent.K2_GetComponentLocation` _characterlocation)))
  (bind _rootcomponent (`Actor.RootComponent` (`self.InteractingActor`)))
  (`parent.StartInteraction` InteractingActor)
  (bind _asnpc_bp (cast `/Game/GymBP/NPC/AI/NPC_BP` (`self.InteractingActor`)))
  (bind _output_get (set `self.Character` _asnpc_bp))
  (`PrimitiveComponent.SetCollisionEnabled` (`self.StaticMesh`) "NoCollision")
  (`|ExecutionSequence`
    (:`then_0`
      (`KismetSystemLibrary.MoveComponentTo` _rootcomponent (`KismetMathLibrary.MakeVector` _returnvalue_x _returnvalue_y (+ _returnvalue_z (`CapsuleComponent.CapsuleHalfHeight` (`Character.CapsuleComponent` (`self.Character`))))) (`SceneComponent.K2_GetComponentRotation` _characterlocation) true true 0.5 true))
    (:`then_1`
      (`|PlayMontage` (`Character.Mesh` _output_get) "/Game/Assetfore/OmarinoSvilupparty/animazioni/parallele/ParalleleANIMMONTAGE.ParalleleANIMMONTAGE"
        (:`OnCompleted`
          (`KismetSystemLibrary.MoveComponentTo` _rootcomponent (+ (`SceneComponent.K2_GetComponentLocation` (`self.CharacterLocationFinale`)) (`KismetMathLibrary.MakeVector` 0.0 0.0 (`CapsuleComponent.CapsuleHalfHeight` (`Character.CapsuleComponent` (`self.Character`))))) (struct) true true)
          (`PrimitiveComponent.SetCollisionEnabled` (`self.StaticMesh`) "QueryAndPhysics")
          (set `self.AzioneCompletata` true)
          (`/Game/Interfaces/InteractGym.EndInteraction`))))))

(event `/Game/Interfaces/InteractGym.EndInteraction`
  (if (`self.AzioneCompletata`)
    (`parent.EndInteraction`)))

(fn `UserConstructionScript`
  (`parent.UserConstructionScript`))