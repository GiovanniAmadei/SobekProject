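; CasseBP is an interactable gym object, apparently speakers, where a character performs a YMCA dance.
; Interaction eases the character to CharacterLocationAttrezzo while playing the montage, whose completion sets AzioneCompletata and lets EndInteraction reach the parent.
; Tick mutes the Soundtrack actor when the camera pawn is within 1000 units, otherwise its clamped-distance multiplier is effectively full volume.
; Destroyed sets that volume back to full.
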(event `self.ReceiveBeginPlay`
  (`parent.ReceiveBeginPlay`))

(event `self.ReceiveTick`
  (params (DeltaSeconds :type "Float (single-precision)"))
  (bind _returnvalue (`GameplayStatics.GetActorOfClass` "/Game/Soundtrack.Soundtrack_C"))
  (bind _asgym_camera_controller (cast `/Game/GymBP/GymCameraController` (`GameplayStatics.GetPlayerController` 0)))
  (bind _returnvalue_2 (`self.GetDistanceTo` (`/Game/GymBP/GymCameraController.CameraPawnRef` _asgym_camera_controller)))
  (if (< _returnvalue_2 1000.0)
    (bind _audio (`/Game/Soundtrack.Audio` _returnvalue))
    (`AudioComponent.SetVolumeMultiplier` _audio 0.0)
    (else
      (`AudioComponent.SetVolumeMultiplier` _audio (`KismetMathLibrary.FClamp` _returnvalue_2)))))

(event `self.ReceiveDestroyed`
  (`AudioComponent.SetVolumeMultiplier` (`/Game/Soundtrack.Audio` (stale `self.ReceiveTick` _returnvalue)) 1.0))

(event `/Game/Interfaces/InteractGym.StartInteraction`
  (params (InteractingActor :type "Character Object Reference"))
  (bind _characterlocationattrezzo (`self.CharacterLocationAttrezzo`))
  (bind (_returnvalue_x _returnvalue_y _returnvalue_z) (`KismetMathLibrary.BreakVector` (`SceneComponent.K2_GetComponentLocation` _characterlocationattrezzo)))
  (`parent.StartInteraction` InteractingActor)
  (bind _output_get (set `self.CharacterAzione` (`self.InteractingActor`)))
  (`|ExecutionSequence`
    (:`then_0`
      (`KismetSystemLibrary.MoveComponentTo` (`Actor.RootComponent` (`self.InteractingActor`)) (`KismetMathLibrary.MakeVector` _returnvalue_x _returnvalue_y (+ _returnvalue_z (`CapsuleComponent.CapsuleHalfHeight` (`Character.CapsuleComponent` (`self.CharacterAzione`))))) (`SceneComponent.K2_GetComponentRotation` _characterlocationattrezzo) true true 0.5))
    (:`then_1`
      (`|PlayMontage` (`Character.Mesh` _output_get) "/Game/Assetfore/OmarinoSvilupparty/animazioni/YMCADANCEANIMMONTAGE.YMCADANCEANIMMONTAGE"
        (:`OnCompleted`
          (set `self.AzioneCompletata` true)
          (`/Game/Interfaces/InteractGym.EndInteraction`))))))

(event `/Game/Interfaces/InteractGym.EndInteraction`
  (if (`self.AzioneCompletata`)
    (`parent.EndInteraction`)))

(fn `UserConstructionScript`
  (`parent.UserConstructionScript`))