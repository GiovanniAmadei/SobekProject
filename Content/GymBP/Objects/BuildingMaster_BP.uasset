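; BuildingMaster_BP is a master building actor that shows or hides an info widget when clicked.
; Its construction script applies the DisplayMesh variable to the static mesh, hides and offsets the widget, and calls AddClickableComponent.
; The ActorOnClicked event uses a Clicked flag to toggle the widget's visibility.
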(event `self.ReceiveActorOnClicked`
  (params (ButtonPressed :type "Key Structure"))
  (bind _widget (`self.Widget`))
  (if (`self.Clicked`)
    (`SceneComponent.SetVisibility` _widget false false)
    (set `self.Clicked` false)
    (else
      (`SceneComponent.SetVisibility` _widget true false)
      (set `self.Clicked` true))))

(fn `UserConstructionScript`
  (bind _widget (`self.Widget`))
  (`StaticMeshComponent.SetStaticMesh` (`self.StaticMesh`) (`self.DisplayMesh`))
  (`SceneComponent.SetVisibility` _widget false false)
  (`SceneComponent.K2_AddLocalOffset` _widget (300.0 0.0 400.0) false false)
  (`AddComponent|NODE_AddClickableComponent-0`))