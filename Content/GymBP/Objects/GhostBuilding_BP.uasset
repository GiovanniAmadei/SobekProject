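; Placement ghost for build mode, previewing the selected building's mesh with a direction arrow and packaging its data as a construction struct.
; ConstructObject spawns a throwaway instance to read building data, feeds it to OnSpawn, then destroys it.
; While active, a gated Tick moves the ghost to a mouse-traced snap box or grid-snapped cursor position.
; Overlap, overlap permission and budget determine blue or red materials, refreshed when overlap state changes.
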(event `OnSpawn`
  (params (DisplayMesh :type "StaticMesh Object Reference") (BuildingClass :type "/Game/GymBP/Objects/BuildingMaster_BP Class Reference") (ConstructionProxy :type "/Game/GymBP/Construction/ConstructionProxy_BP Class Reference") (WorkHours :type "Float (double-precision)") (Costo :type Integer) (Costruzione :type Boolean) (Occupato :type Boolean) (Nome :type Name))
  (bind _arrow (`self.Arrow`))
  ;[1 1 1] OnSpawn Ghost
  (if (not (`self.IsActive`))
    (set `self.BuildingClass` BuildingClass)
    (set `self.ConstructionProxy` ConstructionProxy)
    (set `self.DisplayMesh` DisplayMesh)
    (set `self.WorkHoursRequired` WorkHours)
    (set `self.CostoRichiesto` Costo)
    (set `self.Occupato` Occupato)
    (set `self.Nome` Nome)
    (set `self.PuòOverlap?` Costruzione)
    (set `self.IsActive` true)
    (set `/Game/GymBP/GymCameraController.BuildModeActive` true (`self.ControllerRef`))
    (`StaticMeshComponent.SetStaticMesh` (`self.GhostBuilding_Mesh`) (`self.DisplayMesh`))
    (`self.OpenTickGate`)
    (`self.SetMaterial` (not (`self.IsOverlapping`)))
    (bind _output_get (set `self.Box Extent` (`.BoxExtent` (`KismetSystemLibrary.GetComponentBounds` (`self.GhostBuilding_Mesh`)))))
    (`SceneComponent.K2_SetRelativeLocation` _arrow (`KismetMathLibrary.MakeVector` (.x _output_get)) false false)
    (`SceneComponent.SetHiddenInGame` _arrow false false)
    (`/Game/Libraries/FunctionLibrary.SetBuildingCollisionBox` (`self.Collision`) (`self.GhostBuilding_Mesh`))))

(event `KillGhost`
  ;[1 1 1] Kill Ghost
  (set `self.BuildingClass` null)
  (set `self.ConstructionProxy` null)
  (`self.CloseTickGate`)
  (set `self.DisplayMesh` null)
  (set `self.IsActive` false)
  (set `/Game/GymBP/GymCameraController.BuildModeActive` false (`self.ControllerRef`))
  (`StaticMeshComponent.SetStaticMesh` (`self.GhostBuilding_Mesh`) (`self.DisplayMesh`))
  (`self.K2_SetActorRotation` (struct))
  (`SceneComponent.SetHiddenInGame` (`self.Arrow`) true false))

(event `/Game/Interfaces/GymInterface_Hud.ConstructObject`
  (params (MainObject :type "/Game/GymBP/Objects/BuildingMaster_BP Class Reference") (Costo :type Integer) (Nome :type Name))
  ;[1 1 1] Construct Building
  (bind _returnvalue (`|SpawnActorFromClass` MainObject (`KismetMathLibrary.MakeTransform` (0.0 0.0 0.0)) "AlwaysSpawn" "MultiplyWithRoot" null (`self.ControllerRef`) Costo false Nome null))
  (`|ExecutionSequence`
    (:`then_0`
      (bind _asbuilding_master_bp (castclass `/Game/GymBP/Objects/BuildingMaster_BP` MainObject))
      (`self.KillGhost`)
      (`self.OnSpawn` (`/Game/GymBP/Objects/BuildingMaster_BP.DisplayMesh` _returnvalue) _asbuilding_master_bp (`/Game/GymBP/Objects/BuildingMaster_BP.ConstructionProxy` _returnvalue) (`/Game/GymBP/Objects/BuildingMaster_BP.ConstructionTime` _returnvalue) (`/Game/GymBP/Objects/BuildingMaster_BP.Costo` _returnvalue) (`/Game/GymBP/Objects/BuildingMaster_BP.Costruzione?` _returnvalue) (`/Game/GymBP/Objects/BuildingMaster_BP.Occupato` _returnvalue) (`/Game/GymBP/Objects/BuildingMaster_BP.Nome` _returnvalue)))
    (:`then_1`
      (`self.K2_DestroyActor` _returnvalue))))

(event `self.ReceiveTick`
  (params (DeltaSeconds :type "Float (single-precision)"))
  ;[1 1 1] Tick
  (`/Engine/EditorBlueprintResources/StandardMacros.Gate` true :!label _label
    (:`Exit`
      (`self.K2_SetActorLocation` self (`self.SetGridSnapVector`) false false)
      (if (`self.CheckOverlap`)
        (`self.SetMaterial` true)
        (else
          (`self.SetMaterial` false))))))

(event `OpenTickGate`
  ;[1 1 1] Tick
  (goto _label :!via `Open`))

(event `CloseTickGate`
  ;[1 1 1] Tick
  (goto _label :!via `Close`))

(event `SetMaterial`
  (params (IsError :type Boolean))
  (bind _ghostbuilding_mesh (`self.GhostBuilding_Mesh`))
  (bind _returnvalue (`PrimitiveComponent.GetNumMaterials` _ghostbuilding_mesh))
  (if (not (== IsError (`self.IsOverlapping`)))
    (bind _output_get (set `self.IsOverlapping` IsError))
    (if _output_get
      (if (`self.PuòOverlap?`)
        (for _index (range (+ _returnvalue 1)) :!label _label_2
          ;[1 1 1] Colori relativi all'overlap
          (`PrimitiveComponent.SetMaterial` _ghostbuilding_mesh _index "/Game/MyMaterials/Ghost-Blu.Ghost-Blu"))
        (else
          (for _index_2 (range (+ _returnvalue 1)) :!label _label_3
            ;;[1 1 1] Cambiare colore a ghost red quando si risistema
            (`PrimitiveComponent.SetMaterial` _ghostbuilding_mesh _index_2 "/Game/MyMaterials/Ghost-Red.Ghost-Red"))))
      (elif (`self.CheckBudget`)
        (goto _label_3)
        (else
          (goto _label_2))))))

(fn `CheckBounds`
  (returns (OutOfBounds :type Boolean))
  (return (< (`KismetArrayLibrary.Array_Length` (`self.GetOverlappingActors` "/Script/Engine.BlockingVolume")) 0)))

(fn `CheckBudget`
  (returns (`CostaTroppo?` :type Boolean))
  (return (> (`self.CostoRichiesto`) (`/Game/GymBP/GymCameraController.Soldi` (`self.ControllerRef`)))))

(fn `CheckOverlap`
  (returns (Overlapping :type Boolean))
  (return (> (`KismetArrayLibrary.Array_Length` (`self.GetOverlappingActors` "/Script/Engine.Actor")) 0)))

(fn `DetectBoxes`
  (returns (Found :type Boolean) (Transform :type "Transform Structure"))
  (locals (LocalFound :type Boolean))
  (bind _hit_component (`self.Hit Component`))
  (bind _boxes (message `/Game/Interfaces/BPI_Snap.ReturnBoxes` (`.Hit Actor` (`self.GetHitActorsSnap`))))
  (for _array_element _boxes
    (`KismetSystemLibrary.PrintString` (`KismetSystemLibrary.GetDisplayName` _hit_component))
    (if (== _array_element _hit_component)
      (set `local.LocalFound` true)
      (break)))
  (return (`local.LocalFound`) (`SceneComponent.K2_GetComponentToWorld` (`self.Hit Component`))))

(fn `GetConstructionStruct`
  (returns (ConstructionStruct :type "/Game/Structs/Construction_Struct Structure"))
  (return (make `/Game/Structs/Construction_Struct` (`KismetTextLibrary.Conv_NameToText` (`self.Nome`)) "" (`self.BuildingClass`) (`self.ConstructionProxy`) "NewEnumerator0" (`KismetMathLibrary.MakeTransform` (`self.K2_GetActorLocation`) (`self.K2_GetActorRotation`)) null (`self.DisplayMesh`) (`self.WorkHoursRequired`) (`self.CostoRichiesto`) (`self.Occupato`) (`self.Usura`))))

(fn `GetHitActorsSnap`
  (returns (`Hit Component` :type "PrimitiveComponent Object Reference") (`Hit Actor` :type "Actor Object Reference"))
  (bind (_worldlocation _worlddirection) (`PlayerController.DeprojectMousePositionToWorld` (`GameplayStatics.GetPlayerController` 0)))
  (bind (_outhit _returnvalue) (`KismetSystemLibrary.LineTraceSingle` _worldlocation (+ _worldlocation (* _worlddirection 1000000.0)) "TraceTypeQuery1"))
  (if _returnvalue
    (bind (_bblockinghit _binitialoverlap _time _distance _location _impactpoint _normal _impactnormal _physmat _hitactor _hitcomponent) (`GameplayStatics.BreakHitResult` _outhit))
    (bind _output_get (set `self.Hit Actor` _hitactor))
    (bind _output_get_2 (set `self.Hit Component` _hitcomponent))
    (return _output_get_2 _output_get)))

(fn `ReturnBoxes`
  (returns (Boxes :type "Array of BoxComponent Object Reference"))
  (return))

(fn `SetCalendar`
  (params (Date :type "Array of Integer (by ref)"))
  (returns (Success :type Boolean))
  (return false))

(fn `SetClock`
  (params (Time :type "Array of Integer (by ref)"))
  (returns (Success :type Boolean))
  (return false))

(fn `SetCursorPosition`
  (params (CursorLocation :type "Vector Structure"))
  (set `self.CursorWorldPosition` CursorLocation)
  (return))

(fn `SetGridSnapVector`
  (returns (GridSnap :type "Vector Structure"))
  (bind (_cursorworldposition_x _cursorworldposition_y _cursorworldposition_z) (`KismetMathLibrary.BreakVector` (`self.CursorWorldPosition`)))
  (bind _gridsize (`self.GridSize`))
  (bind (_found _transform) (`self.DetectBoxes`))
  (if _found
    (`KismetSystemLibrary.PrintString` "Hello")
    (return (.location _transform))
    (else
      (return (`KismetMathLibrary.MakeVector` (`/Game/Libraries/FunctionLibrary.GridSnap` _cursorworldposition_x _gridsize) (`/Game/Libraries/FunctionLibrary.GridSnap` _cursorworldposition_y _gridsize) (`/Game/Libraries/FunctionLibrary.GridSnap` _cursorworldposition_z _gridsize))))))

(fn `UserConstructionScript`)