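; Michele_BP is an NPC actor that shows an info panel with its name and description when clicked.
; The construction script creates its own INFONPC widget and stores it as RefWidget.
; On click, if the GymCameraController is not in build mode, it hides the RefInfo widget, hands its widget to the controller, fills in the text and adds it to the viewport.
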(event `self.ReceiveBeginPlay`)

(event `self.ReceiveActorOnClicked`
  (params (ButtonPressed :type "Key Structure"))
  ;[1 1 1] Evitiamo che si attivi il widget dell'oggetto se viene cliccato mentre stiamo piazzando un altro oggetto
  (bind _asgym_camera_controller (cast `/Game/GymBP/GymCameraController` (`GameplayStatics.GetPlayerController` 0)))
  (if (not (`/Game/GymBP/GymCameraController.BuildModeActive` _asgym_camera_controller))
    (`Widget.SetVisibility` (`/Game/GymBP/GymCameraController.RefInfo` _asgym_camera_controller) "Hidden")
    (bind _output_get (set `/Game/GymBP/GymCameraController.RefINFONPC` (`self.RefWidget`) _asgym_camera_controller))
    (bind _refinfonpc (`/Game/GymBP/GymCameraController.RefINFONPC` _asgym_camera_controller))
    (set `/Game/HUDs/INFONPC.Name` (`KismetStringLibrary.Conv_StringToName` (`self.Nome`)) _refinfonpc)
    (set `/Game/HUDs/INFONPC.Descrizione` (`KismetTextLibrary.Conv_StringToText` (`self.Scritta`)) _refinfonpc)
    (`Widget.SetVisibility` _output_get "HitTestInvisible")
    (`UserWidget.AddToViewport` _output_get 0)))

(fn `UserConstructionScript`
  (bind _returnvalue (`|GenericCreateObject` "/Game/HUDs/INFONPC.INFONPC_C"))
  (set `self.RefWidget` _returnvalue))