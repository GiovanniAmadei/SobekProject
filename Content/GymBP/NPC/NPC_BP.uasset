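; Gym NPC Blueprint that gives each character a random identity and toggles its widget when clicked.
; The construction script rolls sex, picks a matching name from enums, stores both in a profile, and hides the offset widget.
; A dynamic material sets body color from a separate random roll, so it can mismatch the stored sex.
; A random wander-and-animate AI loop exists but is disconnected from BeginPlay.
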(event `self.ReceiveActorOnClicked`
  (params (ButtonPressed :type "Key Structure"))
  (if (`self.Clicked`)
    (`SceneComponent.SetVisibility` (`self.Widget`) false false)
    (set `self.Clicked` false)
    (else
      (`SceneComponent.SetVisibility` (`self.Widget`) true false)
      (set `self.Clicked` true))))

(event `self.ReceiveBeginPlay`)

(fn `GetRandomName`
  (params (Sex :type "/Game/Enums/NPCSexType_Enum Enum" :default "NewEnumerator0"))
  (returns (Name :type String))
  (if (`|EnumEquality` Sex "NewEnumerator0")
    (return (`|GetEnumeratorNameAsString` (cast `/Game/Enums/NPCNameMale_Enum` (`KismetMathLibrary.Conv_IntToByte` (`KismetMathLibrary.RandomIntegerInRange` 0 (- (enumcount `/Game/Enums/NPCNameMale_Enum`) 1))))))
    (else
      (return (`|GetEnumeratorNameAsString` (cast `/Game/Enums/NPCNameFemale_Enum` (`KismetMathLibrary.Conv_IntToByte` (`KismetMathLibrary.RandomIntegerInRange` 0 (- (enumcount `/Game/Enums/NPCNameFemale_Enum`) 1)))))))))

(fn `RandomNPCFeatures`
  (locals (MaterialInstance :type "MaterialInstanceDynamic Object Reference") (MaleColor :type "LinearColor Structure" :default (struct :`R` 0.061 :`G` 0.107 :`B` 0.451)) (FemaleColor :type "LinearColor Structure" :default (struct :`R` 0.451 :`G` 0.028 :`B` 0.266)) (`ColorTo Apply` :type "LinearColor Structure") (Sex :type Byte))
  (bind _returnvalue (`KismetMathLibrary.RandomIntegerInRange` 0 1))
  (bind _materialinstance (`local.MaterialInstance`))
  (bind _returnvalue_2 (cast `/Game/Enums/NPCSexType_Enum` (`KismetMathLibrary.Conv_IntToByte` _returnvalue)))
  (bind _returnvalue_3 (`PrimitiveComponent.CreateDynamicMaterialInstance` (`self.Mesh`) 0 "/Game/Characters/Mannequin_UE4/Materials/M_MannequinUE4_Body.M_MannequinUE4_Body" "None"))
  (set `local.MaterialInstance` _returnvalue_3)
  (set `local.Sex` _returnvalue_2)
  (switch `int` _returnvalue
    (:`Default`
      (if (`|EnumEquality` _returnvalue_2 "NewEnumerator0")
        (`MaterialInstanceDynamic.SetVectorParameterValue` _materialinstance "BodyColor" (`local.MaleColor`))
        (else
          (`MaterialInstanceDynamic.SetVectorParameterValue` _materialinstance "BodyColor" (`local.FemaleColor`))))
      (bind _name (`self.GetRandomName` (cast `/Game/Enums/NPCSexType_Enum` (`local.Sex`))))
      (set `self.MyProfile` (make `/Game/Structs/NPCProfile_Struct` _name (cast `/Game/Enums/NPCSexType_Enum` (`local.Sex`))))
      (`KismetSystemLibrary.PrintString` _name))))

(fn `UserConstructionScript`
  (`self.RandomNPCFeatures`)
  (`SceneComponent.K2_AddWorldOffset` (`self.Widget`) (300.0 0.0 400.0) false false)
  (`SceneComponent.SetVisibility` (`self.Widget`) false false))