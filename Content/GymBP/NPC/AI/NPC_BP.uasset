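; Gym customer NPC for a gym management game, with randomized sex, profile and appearance.
; BeginPlay runs a latent macro routine: pay at reception, change clothes, make six Cardio/Power machine visits ordered by profile, then leave.
; Visits claim random available tagged equipment via interface messages and poll completion; waiting drains satisfaction until the member quits.
; NPCs sometimes drink or drop dirt, fall on overlapping dirt, and show info and action widgets when clicked.
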(event `self.ReceiveBeginPlay`
  (bind (_myprofile_name _myprofile_sex _myprofile_gymprofile) (break `/Game/Structs/NPC_Struct` (`self.MyProfile`)))
  (bind _returnvalue (`|GetEnumeratorNameAsString` _myprofile_gymprofile))
  (`self.VaiAReception`
    (:`End`
      (`self.VaiInSpogliatoio`
        (:`Output`
          (if (or (`KismetStringLibrary.EqualEqual_StrStr` _returnvalue "Casual") (`KismetStringLibrary.EqualEqual_StrStr` _returnvalue "Cardio Enthusiast") (`KismetStringLibrary.EqualEqual_StrStr` _returnvalue "Runner"))
            (`self.UsaAttrezzoDellaTuaClasse` "Cardio")
            (`self.UsaAttrezzoDellaTuaClasse` "Cardio")
            (`self.UsaAttrezzoDellaTuaClasse` "Power")
            (`self.UsaAttrezzoDellaTuaClasse` "Cardio")
            (`self.UsaAttrezzoDellaTuaClasse` "Power")
            (`self.UsaAttrezzoDellaTuaClasse` "Cardio")
            (else
              (`self.UsaAttrezzoDellaTuaClasse` "Power")
              (`self.UsaAttrezzoDellaTuaClasse` "Power")
              (`self.UsaAttrezzoDellaTuaClasse` "Cardio")
              (`self.UsaAttrezzoDellaTuaClasse` "Power")
              (`self.UsaAttrezzoDellaTuaClasse` "Cardio")
              (`self.UsaAttrezzoDellaTuaClasse` "Power")))
          (`self.VaiVia`))))))

(event `self.ReceiveActorOnClicked`
  (params (ButtonPressed :type "Key Structure"))
  (bind (_myprofile_name _myprofile_sex _myprofile_gymprofile _myprofile_motivation _myprofile_membershiptype) (break `/Game/Structs/NPC_Struct` (`self.MyProfile`)))
  (`|ExecutionSequence`
    (:`then_0`
      ;[1 1 1] Evitiamo che si attivi il widget dell'oggetto se viene cliccato mentre stiamo piazzando un altro oggetto
      (bind _asgym_camera_controller (cast `/Game/GymBP/GymCameraController` (`GameplayStatics.GetPlayerController` 0)))
      (if (not (`/Game/GymBP/GymCameraController.BuildModeActive` _asgym_camera_controller))
        (`Widget.RemoveFromParent` (`/Game/GymBP/GymCameraController.RefInfo` _asgym_camera_controller))
        (bind _refinfonpc (`/Game/GymBP/GymCameraController.RefINFONPC` _asgym_camera_controller))
        (`Widget.RemoveFromParent` _refinfonpc)
        (bind _output_get (set `/Game/GymBP/GymCameraController.RefINFONPC` (`self.RefWidget`) _asgym_camera_controller))
        (set `/Game/HUDs/INFONPC.NPC` self _output_get)
        (set `/Game/HUDs/INFONPC.Name` (`KismetStringLibrary.Conv_StringToName` _myprofile_name) _refinfonpc)
        (set `/Game/HUDs/INFONPC.Profilo` (`|GetEnumeratorNameAsString` _myprofile_gymprofile) _refinfonpc)
        (`Widget.SetVisibility` _output_get "HitTestInvisible")
        (`UserWidget.AddToViewport` _output_get 0)))
    (:`then_1`
      (bind _returnvalue (`|CreateWidget` "/Game/HUDs/WidgetActionNPC.WidgetActionNPC_C"))
      (set `/Game/HUDs/WidgetActionNPC.NPC` self _returnvalue)
      (`UserWidget.AddToViewport` _returnvalue 0))))

(event `self.CapsuleComponent.OnComponentBeginOverlap`
  (params (OverlappedComponent :type "PrimitiveComponent Object Reference") (OtherActor :type "Actor Object Reference") (OtherComp :type "PrimitiveComponent Object Reference") (OtherBodyIndex :type Integer) (bFromSweep :type Boolean) (SweepResult :type "HitResult Structure (by ref)"))
  ;[1 1 1] Animazione cadi se incroci sporco
  (cast `/Game/GymBP/GameObjects/SporcoBP` OtherActor)
  (`|PlayMontage` (`self.Mesh`) "/Game/Assetfore/OmarinoSvilupparty/animazioni/cadute/FALLFLATANIMMONTAGE.FALLFLATANIMMONTAGE"))

(fn `GetMembership`
  (returns (ReturnValue :type "/Game/Enums/NPC_MembershipType Enum") (String :type String))
  (return (cast `/Game/Enums/NPC_MembershipType` (`KismetMathLibrary.Conv_IntToByte` (`KismetMathLibrary.RandomIntegerInRange` 0 (- (enumcount `/Game/Enums/NPC_MembershipType`) 1)))) ""))

(fn `GetMotivation`
  (returns (ReturnValue :type "/Game/Enums/NPC_Motivation Enum") (String :type String))
  (bind _returnvalue (cast `/Game/Enums/NPC_Motivation` (`KismetMathLibrary.Conv_IntToByte` (`KismetMathLibrary.RandomIntegerInRange` 0 (- (enumcount `/Game/Enums/NPC_Motivation`) 1)))))
  (return _returnvalue (`|GetEnumeratorNameAsString` _returnvalue)))

(fn `GetRandomGymProfile`
  (returns (ReturnValue :type "/Game/Enums/NPC_GymProfile Enum") (String :type String))
  (bind _returnvalue (cast `/Game/Enums/NPC_GymProfile` (`KismetMathLibrary.Conv_IntToByte` (`KismetMathLibrary.RandomIntegerInRange` 0 (- (enumcount `/Game/Enums/NPC_GymProfile`) 1)))))
  (return _returnvalue (`|GetEnumeratorNameAsString` _returnvalue)))

(fn `GetRandomName`
  (params (Sex :type "/Game/Enums/NPCSexType_Enum Enum" :default "NewEnumerator0"))
  (returns (Name :type String))
  (if (`|EnumEquality` Sex "NewEnumerator0")
    (return (`|GetEnumeratorNameAsString` (cast `/Game/Enums/NPCNameMale_Enum` (`KismetMathLibrary.Conv_IntToByte` (`KismetMathLibrary.RandomIntegerInRange` 0 (- (enumcount `/Game/Enums/NPCNameMale_Enum`) 1))))))
    (else
      (return (`|GetEnumeratorNameAsString` (cast `/Game/Enums/NPCNameFemale_Enum` (`KismetMathLibrary.Conv_IntToByte` (`KismetMathLibrary.RandomIntegerInRange` 0 (- (enumcount `/Game/Enums/NPCNameFemale_Enum`) 1)))))))))

(fn `ImpostaNuovoObiettivoAttrezzo`
  (params (Actor :type "/Game/GymBP/Objects/BuildingMaster_BP Object Reference"))
  (returns (Attrezzo :type "/Game/GymBP/Objects/BuildingMaster_BP Object Reference"))
  (bind _output_get (set `self.InteractableObject` Actor))
  (return _output_get))

(fn `ImpostaVestitiCasuali`
  (bind _arraycolorimaglietta (`self.ArrayColoriMaglietta`))
  (`PrimitiveComponent.SetMaterial` (`self.Mesh`) 1 (`KismetArrayLibrary.Array_Random` _arraycolorimaglietta))
  (`PrimitiveComponent.SetMaterial` (`self.Mesh`) 2 (`KismetArrayLibrary.Array_Random` _arraycolorimaglietta))
  (`PrimitiveComponent.SetMaterial` (`self.Mesh`) 3 (`KismetArrayLibrary.Array_Random` _arraycolorimaglietta)))

(fn `ImpostaVestitiPelleECapelliCasuali`
  (bind _arraycolorimaglietta (`self.ArrayColoriMaglietta`))
  (`PrimitiveComponent.SetMaterial` (`self.Mesh`) 1 (`KismetArrayLibrary.Array_Random` _arraycolorimaglietta))
  (`PrimitiveComponent.SetMaterial` (`self.Mesh`) 4 (`KismetArrayLibrary.Array_Random` (`self.ArrayColoriCapelli`)))
  (`PrimitiveComponent.SetMaterial` (`self.Mesh`) 0 (`KismetArrayLibrary.Array_Random` (`self.ArrayPelle`)))
  (`PrimitiveComponent.SetMaterial` (`self.Mesh`) 2 (`KismetArrayLibrary.Array_Random` _arraycolorimaglietta))
  (`PrimitiveComponent.SetMaterial` (`self.Mesh`) 3 (`KismetArrayLibrary.Array_Random` _arraycolorimaglietta)))

(fn `RandomNPCFeatures`
  (locals (MaterialInstance :type "MaterialInstanceDynamic Object Reference") (MaleColor :type "LinearColor Structure" :default (struct :`R` 0.061 :`G` 0.107 :`B` 0.451)) (FemaleColor :type "LinearColor Structure" :default (struct :`R` 0.451 :`G` 0.028 :`B` 0.266)) (`ColorTo Apply` :type "LinearColor Structure") (Sex :type Byte))
  (bind _returnvalue (`KismetMathLibrary.RandomIntegerInRange` 0 1))
  (bind _mesh (`self.Mesh`))
  (bind _returnvalue_2 (cast `/Game/Enums/NPCSexType_Enum` (`KismetMathLibrary.Conv_IntToByte` _returnvalue)))
  (bind _returnvalue_3 (`PrimitiveComponent.CreateDynamicMaterialInstance` (`self.Mesh`) 0 "/Game/Characters/Mannequin_UE4/Materials/M_MannequinUE4_Body.M_MannequinUE4_Body" "None"))
  (set `local.MaterialInstance` _returnvalue_3)
  (set `local.Sex` _returnvalue_2)
  (switch `int` _returnvalue
    (:`Default`
      (if (`|EnumEquality` _returnvalue_2 "NewEnumerator0")
        (`SkeletalMeshComponent.SetSkeletalMeshAsset` _mesh "/Game/Assetfore/OmarinoSvilupparty/convestiti/omarino_vestito_svilupparty.omarino_vestito_svilupparty")
        (`SkeletalMeshComponent.SetSkeletalMeshAsset` (`self.Mesh`) "/Game/Assetfore/OmarinoSvilupparty/livelli/4/4.4")
        (else
          (`SkeletalMeshComponent.SetSkeletalMeshAsset` _mesh "/Game/Assetfore/personaggi/donna/donna_T-Pose.donna_T-Pose")
          (`SkeletalMeshComponent.SetSkeletalMeshAsset` (`self.Mesh`) "/Game/Assetfore/personaggi/donna/livelli/4/4.4")))
      (bind _name (`self.GetRandomName` (cast `/Game/Enums/NPCSexType_Enum` (`local.Sex`))))
      (set `self.MyProfile` (make `/Game/Structs/NPC_Struct` _name (cast `/Game/Enums/NPCSexType_Enum` (`local.Sex`)) (`self.GetRandomGymProfile`) (`self.GetMotivation`) (`self.GetMembership`) (`KismetMathLibrary.RandomIntegerInRange` 12 60)))
      (`self.ImpostaVestitiPelleECapelliCasuali`))))

(fn `SetIsBusy`
  (params (IsBusy :type Boolean))
  (`BlackboardComponent.SetValueAsBool` (`AIBlueprintHelperLibrary.GetBlackboard` (`self.AiControllerRef`)) (`self.IsBusy`) IsBusy)
  (return))

(fn `UserConstructionScript`
  (`self.RandomNPCFeatures`)
  (bind _returnvalue (`|GenericCreateObject` "/Game/HUDs/INFONPC.INFONPC_C"))
  (set `self.RefWidget` _returnvalue))