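; Construction proxy actor that stands in for a building while it is being built in the gym game.
; The construction script applies the display mesh and fits the entrance and collision box to it.
; Each tick advances a clockwork counter scaled by the game state's time unit, kept in sync with game-speed changes.
; When work time reaches the construction time set from work hours, it broadcasts completion and destroys itself shortly after.
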(event `self.ReceiveBeginPlay`
  (bind _output_get (set `self.As Gym Game State` (cast `/Game/GymBP/GymGameState` (`GameplayStatics.GetGameState`) :!pure true)))
  (set `self.TimeUnit` (`/Game/GymBP/GymGameState.TimeUnit` _output_get))
  (add `/Game/GymBP/GymGameState.UpdateGameSpeed` _output_get (delegate `AdjustTime`)))

(event `self.ReceiveTick`
  (params (DeltaSeconds :type "Float (single-precision)"))
  (set `self.Delta` DeltaSeconds)
  (if (not (`self.IsConstructionComplete`))
    (`self.DoWork`)
    (if (>= (`self.WorkTimeSpent`) (`self.ConstructionTime`))
      (set `self.IsConstructionComplete` true)
      (`self.ConstructionCompleted` self)
      (`KismetSystemLibrary.Delay` 0.2)
      (`self.K2_DestroyActor`))))

(event `AdjustTime`
  (params (TimeUnit :type "Float (double-precision)"))
  (set `self.TimeUnit` TimeUnit))

(fn `DoWork`
  (bind _output_get (set `self.Clockwork` (`/Game/Libraries/FunctionLibrary.SetClockwork` (`self.Delta`) (`self.TimeUnit`) (`self.Clockwork`))))
  (set `self.WorkTimeSpent` (* _output_get 60.0))
  (return))

(fn `SetConstructionTime`
  (params (WorkHours :type "Float (double-precision)"))
  (set `self.ConstructionTime` (* WorkHours 60.0))
  (return))

(fn `UserConstructionScript`
  (bind _staticmesh (`self.StaticMesh`))
  (`StaticMeshComponent.SetStaticMesh` _staticmesh (`self.DisplayMesh`))
  (`PrimitiveComponent.SetMaterial` _staticmesh 0 null)
  (`/Game/Libraries/FunctionLibrary.SetBuildingEntrance` (`self.Entrance`) (`self.StaticMesh`))
  (`/Game/Libraries/FunctionLibrary.SetBuildingCollisionBox` (`self.Collision`) (`self.StaticMesh`)))