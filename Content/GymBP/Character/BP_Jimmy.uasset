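; BP_Jimmy is a gym NPC character that can walk to a destination and be clicked to show NPC info.
; GoToTarget sends it to a given location with AIMoveTo.
; On click, outside build mode, it hides the GymCameraController's info widget and shows the NPC info widget named "Gymmy".
; The build mode check keeps clicks made while placing objects from opening the widget.
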(event `GoToTarget`
  (params (TargetLocation :type "Vector Structure"))
  (`|AIMoveTo` self TargetLocation null))

(event `self.ReceiveActorOnClicked`
  (params (ButtonPressed :type "Key Structure"))
  ;[1 1 1] Evitiamo che si attivi il widget dell'oggetto se viene cliccato mentre stiamo piazzando un altro oggetto
  (bind _asgym_camera_controller (cast `/Game/GymBP/GymCameraController` (`GameplayStatics.GetPlayerController` 0)))
  (if (not (`/Game/GymBP/GymCameraController.BuildModeActive` _asgym_camera_controller))
    (`Widget.SetVisibility` (`/Game/GymBP/GymCameraController.RefInfo` _asgym_camera_controller) "Hidden")
    (bind _refinfonpc (`/Game/GymBP/GymCameraController.RefINFONPC` _asgym_camera_controller))
    (set `/Game/HUDs/INFONPC.Name` "Gymmy" _refinfonpc)
    (`Widget.SetVisibility` _refinfonpc "HitTestInvisible")
    (`UserWidget.AddToViewport` _refinfonpc 0)))

(fn `UserConstructionScript`)